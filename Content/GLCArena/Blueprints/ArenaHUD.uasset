(event EventDrawHUD
  (params (SizeX :type Integer) (SizeY :type Integer))
  (bind _returnvalue (Utilities|Text|MakeLiteralText "Game Lost Crash 2015.03"))
  (bind _startup_font (Variables|Default|GetStartup%20Font))
  (bind _returnvalue_2 (Utilities|String|ToString(Text) _returnvalue))
  ;[1 1 1] Show GLC Version at Bottom Left
  (HUD|DrawText (HUD|GetHUD (Game|GetPlayerController 0)) _returnvalue_2 "(R=0.885000,G=0.345506,B=0.119475,A=1.000000)" 0.0 (- (Math|Conversions|ToFloat(Integer) SizeY) (.OutHeight (Class|HUD|GetTextSize _returnvalue_2 _startup_font 1.0))) _startup_font 1.0 false)
  ;[0.6767 1 0.5658] Print out a message when we hit the bounding box
  (Utilities|FlowControl|Gate true
    (:Exit
      (HUD|DrawText "You discovered a secret!" "(R=0.825000,G=0.211164,B=0.761019,A=1.000000)" 0.0 1e+02 "/Game/GLCArena/Textures/Krungthep12.Krungthep12" 1.0 false))))

(event EventCollisionDebugText
  (params (Collision? :type Boolean))
  ;[0.6767 1 0.5658] Print out a message when we hit the bounding box
  (if Collision?
    (Utilities|FlowControl|Gate true) ; enters at Open
    (else
      (Utilities|FlowControl|Gate true) ; enters at Close
    )))

(fn ConstructionScript)