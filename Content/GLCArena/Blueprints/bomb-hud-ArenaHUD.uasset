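; Arena HUD Blueprint that draws a version label, a center crosshair and a bottom-center bar with three bomb cells.
; DrawHUD computes the layout from screen size and literal values, with cells independent of bomb count.
; CollisionDebugText opens or closes a Gate that lets DrawHUD show a secret-discovered message.
; BombEvent_Spent switches on bomb count to identical ToggleVisibility and DrawRect calls outside DrawHUD, apparently unfinished.
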(event Custom|BombEvent_Spent
  (params (BombCount :type Integer))
  (switch int BombCount
    (:1
      (Rendering|ToggleVisibility false)
      (HUD|DrawRect "(R=0,G=0,B=0,A=1)" 0.0 0.0 4e+01 0.0))
    (:2
      (Rendering|ToggleVisibility false)
      (HUD|DrawRect "(R=0,G=0,B=0,A=1)" 0.0 0.0 4e+01 0.0))
    (:3
      (Rendering|ToggleVisibility false)
      (HUD|DrawRect "(R=0,G=0,B=0,A=1)" 0.0 0.0 4e+01 0.0))))

(event EventDrawHUD
  (params (SizeX :type Integer) (SizeY :type Integer))
  (bind _returnvalue (/ SizeY 2))
  (bind _returnvalue_2 (/ SizeX 2))
  (bind _returnvalue_3 (Utilities|Text|MakeLiteralText "Game Lost Crash 2015.03"))
  (bind _returnvalue_4 (/ SizeX 2))
  (bind _returnvalue_5 (Class|KismetSystemLibrary|MakeLiteralInteger 250))
  (bind _returnvalue_6 (Class|KismetSystemLibrary|MakeLiteralInteger 50))
  (bind _returnvalue_7 (Class|KismetSystemLibrary|MakeLiteralInteger 3))
  (bind _returnvalue_8 (Class|KismetSystemLibrary|MakeLiteralInteger 10))
  (bind _startup_font (Variables|Default|GetStartup%20Font))
  (bind _returnvalue_9 (Math|Conversions|ToFloat(Integer) _returnvalue_2))
  (bind _returnvalue_10 (Math|Conversions|ToFloat(Integer) _returnvalue))
  (bind _returnvalue_11 (Utilities|String|ToString(Text) _returnvalue_3))
  (bind _returnvalue_12 (- SizeY _returnvalue_6))
  (bind _returnvalue_13 (/ _returnvalue_5 2))
  (bind _returnvalue_14 (+ _returnvalue_7 1))
  (bind _returnvalue_15 (* _returnvalue_8 2))
  (bind _returnvalue_16 (- _returnvalue_4 _returnvalue_13))
  (bind _returnvalue_17 (- _returnvalue_6 _returnvalue_15))
  (bind _returnvalue_18 (* _returnvalue_14 _returnvalue_8))
  (bind _returnvalue_19 (+ _returnvalue_12 _returnvalue_8))
  (bind _returnvalue_20 (- _returnvalue_5 _returnvalue_18))
  (bind _returnvalue_21 (Math|Conversions|ToFloat(Integer) _returnvalue_19))
  (bind _returnvalue_22 (Math|Conversions|ToFloat(Integer) _returnvalue_17))
  (bind _returnvalue_23 (+ _returnvalue_16 _returnvalue_8))
  (bind _returnvalue_24 (/ _returnvalue_20 _returnvalue_7))
  (bind _returnvalue_25 (+ _returnvalue_23 _returnvalue_8))
  (bind _returnvalue_26 (Math|Conversions|ToFloat(Integer) _returnvalue_24))
  (bind _returnvalue_27 (+ _returnvalue_24 _returnvalue_25))
  ;[1 1 1] Show GLC Version at Bottom Left
  (HUD|DrawText (HUD|GetHUD (Game|GetPlayerController 0)) _returnvalue_11 "(R=0.885000,G=0.345506,B=0.119475,A=1.000000)" 0.0 (- (Math|Conversions|ToFloat(Integer) SizeY) (.OutHeight (Class|HUD|GetTextSize _returnvalue_11 _startup_font 1.0))) _startup_font 1.0 false)
  ;[1 0.285 0.2277] Draw the Crosshair at the center of the screen
  (Class|HUD|DrawLine (- _returnvalue_9 1e+01) _returnvalue_10 (+ _returnvalue_9 1e+01) _returnvalue_10 "(R=0.905000,G=0.226190,B=0.234832,A=1.000000)")
  (Class|HUD|DrawLine _returnvalue_9 (- _returnvalue_10 1e+01) _returnvalue_9 (+ _returnvalue_10 1e+01) "(R=0.780000,G=0.124614,B=0.139512,A=1.000000)")
  ;[1 1 1] Draw Bomb Rectangle Background
  (HUD|DrawRect "(R=0.850000,G=0.055250,B=0.055250,A=1.000000)" (Math|Conversions|ToFloat(Integer) _returnvalue_16) (Math|Conversions|ToFloat(Integer) _returnvalue_12) (Math|Conversions|ToFloat(Integer) _returnvalue_5) (Math|Conversions|ToFloat(Integer) _returnvalue_6))
  ;[1 1 1] Cell 1 - Rect
  (HUD|DrawRect "(R=0,G=0,B=0,A=1)" (Math|Conversions|ToFloat(Integer) _returnvalue_23) _returnvalue_21 _returnvalue_26 _returnvalue_22)
  ;[1 1 1] Cell 2 - Rect
  (HUD|DrawRect "(R=0,G=0,B=0,A=1)" (Math|Conversions|ToFloat(Integer) _returnvalue_27) _returnvalue_21 _returnvalue_26 _returnvalue_22)
  ;[1 1 1] Cell 3 - Rect
  (HUD|DrawRect "(R=0,G=0,B=0,A=1)" (Math|Conversions|ToFloat(Integer) (+ _returnvalue_24 (+ _returnvalue_27 _returnvalue_8))) _returnvalue_21 _returnvalue_26 _returnvalue_22)
  ;[0.6767 1 0.5658] Print out a message when we hit the bounding box
  (Utilities|FlowControl|Gate true
    (:Exit
      (HUD|DrawText "You discovered a secret!" "(R=0.825000,G=0.211164,B=0.761019,A=1.000000)" 0.0 1e+02 "/Game/GLCArena/Textures/Krungthep12.Krungthep12" 1.0 false))))

(event EventCollisionDebugText
  (params (Collision? :type Boolean))
  ;[0.6767 1 0.5658] Print out a message when we hit the bounding box
  (if Collision?
    (Utilities|FlowControl|Gate true) ; enters at Open
    (else
      (Utilities|FlowControl|Gate true) ; enters at Close
    )))

(fn ConstructionScript)